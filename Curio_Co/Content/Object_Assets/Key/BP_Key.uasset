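; BP_Key is a key pickup that the player collects by interacting with it.
; Interactwith adds the item to the interactor's InventorySystem and appends KeyName to the KeyInventory of player 0's BP_PlayerCharacter.
; It then looks up the item's data table row through ItemDataComponent, prints a pickup message and destroys itself.
; LookAt uses the same row lookup to return a "Pick up" prompt with the item's name.
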(event EventBeginPlay)

(event Collision|EventActorBeginOverlap
  (params (OtherActor :type Actor%20Object%20Reference)))

(event EventTick
  (params (DeltaSeconds :type Float%20%28single-precision%29)))

(event EventInteractwith
  (params (PlayerCharacter :type BP%20Player%20Character%20Object%20Reference))
  (bind _itemdatacomponent (Variables|Default|GetItemDataComponent))
  (bind _itemdatacomponent_2 (Variables|Default|GetItemDataComponent))
  (bind _itemid (Variables|/Game/Inventory/ItemDataComponent.ItemDataComponent_C|GetItemID _itemdatacomponent))
  (if true
    (Default|AddtoInventory (Actor|GetComponentbyClass PlayerCharacter "/Game/Inventory/InventorySystem.InventorySystem_C") (.rowname (Variables|/Game/Inventory/ItemDataComponent.ItemDataComponent_C|GetItemID _itemdatacomponent_2)) (Variables|/Game/Inventory/ItemDataComponent.ItemDataComponent_C|GetQuantity _itemdatacomponent_2))
    (bind _asbp_player_character (Utilities|Casting|CastToBP_PlayerCharacter (Game|GetPlayerCharacter 0)))
    (Utilities|Array|Add (Variables|/Game/FP_Character/BP_PlayerCharacter.BP_PlayerCharacter_C|GetKeyInventory _asbp_player_character) (Variables|Default|GetKeyName))
    (bind _returnvalue (Utilities|GetDataTableRow (.datatable _itemid) (.rowname _itemid))
      (:then
        (Development|PrintString (Utilities|String|ToString(Text) (Utilities|Text|FormatText "Picked up {item}" (.Name (Utilities|Struct|BreakItemStructure _returnvalue))))))))
  (Actor|DestroyActor))

(fn ConstructionScript)

(fn Lookat
  (bind _itemdatacomponent (Variables|Default|GetItemDataComponent))
  (bind _itemid (Variables|/Game/Inventory/ItemDataComponent.ItemDataComponent_C|GetItemID _itemdatacomponent))
  (bind _returnvalue (Utilities|GetDataTableRow (.datatable _itemid) (.rowname _itemid))
    (:then
      (return (Utilities|Text|FormatText "Pick up {item}" (.Name (Utilities|Struct|BreakItemStructure _returnvalue)))))))