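; Stealable purple ring pickup that shows a "Steal" prompt when looked at and can be taken through interaction.
; LookAt builds the prompt from the row referenced by its ItemDataComponent, while Interactwith uses a hard-coded Item_Data row.
; If that row's description reads "Stealable", it marks the matching player-controller ActiveQuestList entry stolen, decrements its quantity, and destroys the actor.
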(event EventBeginPlay)

(event Collision|EventActorBeginOverlap
  (params (OtherActor :type Actor%20Object%20Reference)))

(event EventTick
  (params (DeltaSeconds :type Float%20%28single-precision%29)))

(event EventInteractwith
  (params (PlayerCharacter :type BP%20Player%20Character%20Object%20Reference))
  (bind _returnvalue (Utilities|GetDataTableRow "/Game/Inventory/Item_Data.Item_Data" "ring_purple")
    (:then
      (if (Utilities|Enum|Equal(Enum) (Utilities|String|ToString(Text) (.Description (Utilities|Struct|BreakItemStructure _returnvalue))) "Stealable")
        ;[0.15 0.15 0.15 0.5] connect to Loot list
        (bind _asbp_player_controller (Utilities|Casting|CastToBP_PlayerController (Game|GetPlayerController 0)))
        (bind (_array_element _array_index) (Utilities|Array|ForEachLoopwithBreak (Variables|/Game/FP_Character/BP_PlayerController.BP_PlayerController_C|GetActiveQuestList _asbp_player_controller) :!label _label)
          (:LoopBody
            (if (Utilities|Enum|Equal(Enum) (.ItemRowName (Utilities|Struct|BreakS_Loot_Item _array_element)) (Variables|Default|GetTargetItemName))
              (Utilities|Array|SetArrayElem (Variables|/Game/FP_Character/BP_PlayerController.BP_PlayerController_C|GetActiveQuestList _asbp_player_controller) _array_index (Utilities|Struct|MakeS_Loot_Item "ring_purple" true (- (.Quantity (Utilities|Struct|BreakS_Loot_Item _array_element)) 1)))
              (goto _label Break)))
          (:Completed
            (Actor|DestroyActor self)
            (Development|PrintString "Item Stolen")))
        (else
          (Development|PrintString "Can't find item in data table"))))))

(fn ConstructionScript)

(fn Lookat
  (bind _itemdatacomponent (Variables|Default|GetItemDataComponent))
  (bind _itemid (Variables|/Game/Inventory/ItemDataComponent.ItemDataComponent_C|GetItemID _itemdatacomponent))
  (bind _returnvalue (Utilities|GetDataTableRow (.datatable _itemid) (.rowname _itemid))
    (:then
      (return (Utilities|Text|FormatText "Steal {item}" (.Name (Utilities|Struct|BreakItemStructure _returnvalue)))))))