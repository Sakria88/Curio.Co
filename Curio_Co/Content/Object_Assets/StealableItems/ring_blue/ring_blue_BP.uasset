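; Blueprint for the blue ring, a stealable pickup item the player can look at and interact with.
; Interacting reads the hardcoded "ring_blue" row from Item_Data and, if its Description equals "Stealable", prints a message and destroys the actor.
; LookAt builds a "Pick up" prompt from the item name, using the row referenced by its ItemDataComponent instead of the hardcoded one.
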(event EventBeginPlay)

(event Collision|EventActorBeginOverlap
  (params (OtherActor :type Actor%20Object%20Reference)))

(event EventTick
  (params (DeltaSeconds :type Float%20%28single-precision%29)))

(event EventInteractwith
  (params (PlayerCharacter :type BP%20Player%20Character%20Object%20Reference))
  (bind _returnvalue (Utilities|GetDataTableRow "/Game/Inventory/Item_Data.Item_Data" "ring_blue")
    (:then
      (if (Utilities|Enum|Equal(Enum) (Utilities|String|ToString(Text) (.Description (Utilities|Struct|BreakItemStructure _returnvalue))) "Stealable")
        (Development|PrintString "Item Stolen")
        (Actor|DestroyActor self)
        (else
          (Development|PrintString "Can't find item"))))))

(fn ConstructionScript)

(fn Lookat
  (bind _itemdatacomponent (Variables|Default|GetItemDataComponent))
  (bind _itemid (Variables|/Game/Inventory/ItemDataComponent.ItemDataComponent_C|GetItemID _itemdatacomponent))
  (bind _returnvalue (Utilities|GetDataTableRow (.datatable _itemid) (.rowname _itemid))
    (:then
      (return (Utilities|Text|FormatText "Pick up {item}" (.Name (Utilities|Struct|BreakItemStructure _returnvalue)))))))