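; ChocBar_BP is a chocolate bar consumable pickup that the player can look at and interact with to collect.
; LookAt builds a "Pick up" prompt from the item name in the data table row referenced by its ItemDataComponent.
; After a short delay, Interactwith adds the item ID and quantity to the player's InventorySystem.
; If the row is found, it then prints a pickup message and destroys the actor.
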(event EventBeginPlay
  (bind _returnvalue (Actor|GetComponentbyClass "/Game/Inventory/ItemDataComponent.ItemDataComponent_C"))
  (Variables|Default|SetCachedComponent _returnvalue))

(event EventInteractwith
  (params (PlayerCharacter :type BP%20Player%20Character%20Object%20Reference))
  (bind _itemdatacomponent (Variables|Default|GetItemDataComponent))
  (bind _itemdatacomponent_2 (Variables|Default|GetItemDataComponent))
  (bind _itemid (Variables|/Game/Inventory/ItemDataComponent.ItemDataComponent_C|GetItemID _itemdatacomponent))
  (Utilities|FlowControl|Delay 0.4)
  (Default|AddtoInventory (Actor|GetComponentbyClass PlayerCharacter "/Game/Inventory/InventorySystem.InventorySystem_C") (.rowname (Variables|/Game/Inventory/ItemDataComponent.ItemDataComponent_C|GetItemID _itemdatacomponent_2)) (Variables|/Game/Inventory/ItemDataComponent.ItemDataComponent_C|GetQuantity _itemdatacomponent_2))
  (bind _returnvalue (Utilities|GetDataTableRow (.datatable _itemid) (.rowname _itemid))
    (:then
      (Development|PrintString (Utilities|String|ToString(Text) (Utilities|Text|FormatText "Picked up {item}" (.Name (Utilities|Struct|BreakItemStructure _returnvalue)))))
      (Actor|DestroyActor))))

(fn ConstructionScript)

(fn Lookat
  (bind _itemdatacomponent (Variables|Default|GetItemDataComponent))
  (bind _itemid (Variables|/Game/Inventory/ItemDataComponent.ItemDataComponent_C|GetItemID _itemdatacomponent))
  (bind _returnvalue (Utilities|GetDataTableRow (.datatable _itemid) (.rowname _itemid))
    (:then
      (return (Utilities|Text|FormatText "Pick up {item}" (.Name (Utilities|Struct|BreakItemStructure _returnvalue)))))))