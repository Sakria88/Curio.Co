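; BP_JackInTheBox is an interactable jack-in-the-box that offers an "Open Box" prompt through LookAt.
; Interactwith sets HasBeenTriggered, then plays one-shot animations on the box, handle and jack meshes together.
; All three branches feed one shared 10-second delay, after which the actor destroys itself.
; HasBeenTriggered is never checked here, and the leftover enemy-interaction and player-message nodes are disconnected.
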(event EventBeginPlay)

(event Collision|EventActorBeginOverlap
  (params (OtherActor :type Actor%20Object%20Reference)))

(event EventTick
  (params (DeltaSeconds :type Float%20%28single-precision%29)))

(event EventInteractwith
  (params (PlayerCharacter :type BP%20Player%20Character%20Object%20Reference))
  (Variables|Default|SetHasBeenTriggered true)
  (Utilities|FlowControl|Sequence
    (:then_0
      (Audio|Components|Audio|Play (Variables|Default|GetBoxMesh) false))
    (:then_1
      (Audio|Components|Audio|Play (Variables|Default|GetHandleMesh) false))
    (:then_2
      (Audio|Components|Audio|Play (Variables|Default|GetJackMesh) false)))
  (Utilities|FlowControl|Delay 1e+01)
  (Actor|DestroyActor))

(fn ConstructionScript)

(fn Lookat
  (return "Open Box"))